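; Master gun weapon Blueprint whose use raises a scaling force field with pulsing and click audio.
; Use and EndUse call multicast start and end events, with starting blocked while overheated.
; A single timeline drives the field's scale and pulse volume, reversing when use ends.
; On drop, the weapon destroys itself after a delay unless it is held again.
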(event `self.ReceiveBeginPlay`
  ;[0.06432 1 0.1783] Begin Play
  (`parent.ReceiveBeginPlay`))

(event `StartFireWeapon_Multicast`
  ;[1 1 1] Fire Weapon
  (if (not (`self.IsOverheated`))
    (`AudioComponent.Play` (`self.AudioPulsate`) 0.0)
    (`AudioComponent.Play` (`self.AudioClick`) 0.0)
    (bind (_direction _animation) (`Timeline|ShieldAnimationTImeline` :!label _label)
      (:`Update`
        (`SceneComponent.SetRelativeScale3D` (`self.ForeField`) (`KismetMathLibrary.MakeVector` _animation _animation _animation))
        (`AudioComponent.SetVolumeMultiplier` (`self.AudioPulsate`) _animation)))))

(event `/Game/Blueprints/Grippable_Interaction.Use`
  ;[1 1 1] Fire Weapon
  (`/Engine/EditorBlueprintResources/StandardMacros.IsValid` (`self.GetOwner`)
    (:`Is Valid`
      (`self.StartFireWeapon_Multicast`))
    (:`Is Not Valid`
      (`self.EndFireWeapon_Multicast`))))

(event `/Game/Blueprints/Grippable_Interaction.EndUse`
  ;[1 1 1] Fire Weapon
  (`self.EndFireWeapon_Multicast`))

(event `EndFireWeapon_Multicast`
  ;[1 1 1] Fire Weapon
  (`AudioComponent.Play` (`self.AudioClick`) 0.0)
  (`AudioComponent.Stop` (`self.AudioPulsate`))
  (goto _label :!via `Reverse`))

(event `/Game/Blueprints/Grippable_Interaction.Drop`
  ;[1 1 1] Fire Weapon
  (`KismetSystemLibrary.Delay` 10.0)
  (bind (_holdingcontrollers _bisheld) (`self.IsHeld`))
  (if (not _bisheld)
    (`self.K2_DestroyActor`)))

(fn `UserConstructionScript`
  (`parent.UserConstructionScript`))