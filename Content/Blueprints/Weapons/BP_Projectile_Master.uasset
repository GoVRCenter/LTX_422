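; Master team-based laser projectile that deals point or radial damage on its first overlap.
; Construction script randomizes launch spread and sets team material and damage type; OnRep_Team reapplies the material on replication.
; Overlap calls ForceClientDamage, which spawns team-tinted impact FX and sound, starts delayed destruction and applies Red or Blue damage types, with none for Friendly.
; Bot hit-reaction and physics-impulse logic is present but disconnected.
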(event `self.ReceiveBeginPlay`
  ;[0.4393 1 0.4971] Begin
  (`GameplayStatics.SpawnSoundAtLocation` (`self.FireSoundFX`) (`self.K2_GetActorLocation`) (struct) 1.0 1.0 0.0 "/Game/Audio/SoundAttenuation_Normal.SoundAttenuation_Normal" "/Game/Audio/NormalSoundConcurrency.NormalSoundConcurrency")
  (if (`self.StartDacayImmediately`)
    (`self.DestroyAmmo`)))

(event `DestroyAmmo`
  (`KismetSystemLibrary.Delay` (`self.DestroyDelay`)) ; Let it finish this frame before we kill it
  (`self.K2_DestroyActor`) ; Then destroy this projectile
)

(event `self.StaticMesh.OnComponentBeginOverlap`
  (params (OverlappedComponent :type "PrimitiveComponent Object Reference") (OtherActor :type "Actor Object Reference") (OtherComp :type "PrimitiveComponent Object Reference") (OtherBodyIndex :type Integer) (bFromSweep :type Boolean) (SweepResult :type "HitResult Structure (by ref)"))
  ;[1 1 1] Hit event with option to apply physics impulse to target actor
  (`/Engine/EditorBlueprintResources/StandardMacros.DoOnce` false
    (:`Completed`
      (if bFromSweep
        (`self.ForceClientDamage` (`self.IsDamageRadial`) OtherActor (`.Location` (`GameplayStatics.BreakHitResult` SweepResult)) (`self.Team`))
        (else
          (`self.ForceClientDamage` (`self.IsDamageRadial`) OtherActor (`self.K2_GetActorLocation`) (`self.Team`)))))))

(event `ForceClientDamage`
  (params (IsRadialDamage :type Boolean) (Actor :type "Actor Object Reference") (Origin :type "Vector Structure") (Team :type "/Game/Blueprints/DATA/Enum_Teams Enum" :default "NewEnumerator0"))
  (bind _returnvalue (`self.GetOwner` Actor))
  (bind _damageradius (`self.DamageRadius`))
  (bind _damageradius_2 (`self.DamageRadius`))
  ;[1 1 1] Hit event with option to apply physics impulse to target actor
  (bind _returnvalue_2 (`GameplayStatics.SpawnEmitterAtLocation` (`self.ParticleEffect`) Origin))
  (switch `/Game/Blueprints/DATA/Enum_Teams` Team
    (:`NewEnumerator0`
      (`ParticleSystemComponent.SetVectorParameter` _returnvalue_2 "Color" (1.0 0.0 0.0)))
    (:`NewEnumerator1`
      (`ParticleSystemComponent.SetVectorParameter` _returnvalue_2 "Color" (0.0 0.0 1.0)))
    (:`NewEnumerator2`
      (`ParticleSystemComponent.SetVectorParameter` _returnvalue_2 "Color" (1.0 1.0 1.0))))
  (`GameplayStatics.SpawnSoundAtLocation` (`self.HitSoundFX`) Origin (struct) 0.5 (`KismetMathLibrary.RandomFloatInRange` 0.9 1.1) 0.0 "/Game/Audio/SoundAttenuation_Normal.SoundAttenuation_Normal" "/Game/Audio/NormalSoundConcurrency.NormalSoundConcurrency")
  (`self.DestroyAmmo`)
  (switch `/Game/Blueprints/DATA/Enum_Teams` Team
    (:`NewEnumerator0`
      (if IsRadialDamage
        (`GameplayStatics.ApplyRadialDamageWithFalloff` :`BaseDamage` (`self.DamageAmount`) :`MinimumDamage` 1.0 :`Origin` Origin :`DamageInnerRadius` (* _damageradius 0.1) :`DamageOuterRadius` _damageradius :`DamageFalloff` 1.0 :`DamageTypeClass` "/Game/Blueprints/Weapons/DamageType_Explosion_RedTeam.DamageType_Explosion_RedTeam_C" :`DamageCauser` _returnvalue :`InstigatedByController` null :`DamagePreventionChannel` "ECC_WorldStatic")
        (else
          (`GameplayStatics.ApplyDamage` Actor (`self.DamageAmount`) null _returnvalue "/Game/Blueprints/Weapons/Damage_RedTeam.Damage_RedTeam_C"))))
    (:`NewEnumerator1`
      (if IsRadialDamage
        (`GameplayStatics.ApplyRadialDamageWithFalloff` :`BaseDamage` (`self.DamageAmount`) :`MinimumDamage` 1.0 :`Origin` Origin :`DamageInnerRadius` (* _damageradius_2 0.1) :`DamageOuterRadius` _damageradius_2 :`DamageFalloff` 1.0 :`DamageTypeClass` "/Game/Blueprints/Weapons/DamageType_Explosion_BlueTeam.DamageType_Explosion_BlueTeam_C" :`DamageCauser` _returnvalue :`InstigatedByController` null :`DamagePreventionChannel` "ECC_WorldStatic")
        (else
          (`GameplayStatics.ApplyDamage` Actor (`self.DamageAmount`) null _returnvalue "/Game/Blueprints/Weapons/Damage_BlueTeam.Damage_BlueTeam_C"))))))

(fn `OnRep_Team`
  (bind _staticmesh (`self.StaticMesh`))
  (switch `/Game/Blueprints/DATA/Enum_Teams` (`self.Team`)
    (:`NewEnumerator0`
      (`PrimitiveComponent.SetMaterial` _staticmesh 0 "/Game/Materials/MI_LaserAnimated_Red.MI_LaserAnimated_Red"))
    (:`NewEnumerator1`
      (`PrimitiveComponent.SetMaterial` _staticmesh 0 "/Game/Materials/MI_LaserAnimated_Blue.MI_LaserAnimated_Blue"))))

(fn `UserConstructionScript`
  (bind _staticmesh (`self.StaticMesh`))
  (bind _accuracydeviation (`self.AccuracyDeviation`))
  (`AudioComponent.SetPitchMultiplier` (`self.SoundFX_Constant`) (`KismetMathLibrary.RandomFloatInRange` 0.96 1.0))
  ;[1 1 1] Set Launch Velocity
  (set `MovementComponent.Velocity` (`KismetMathLibrary.MakeVector` (`self.LaunchVelocity`) (`KismetMathLibrary.RandomFloatInRange` (* _accuracydeviation -1.0) _accuracydeviation) (`KismetMathLibrary.RandomFloatInRange` (* _accuracydeviation -1.0) _accuracydeviation)) (`self.Projectile`))
  ;[1 1 1] SetMaterial
  (switch `/Game/Blueprints/DATA/Enum_Teams` (`self.Team`)
    (:`NewEnumerator0`
      (`PrimitiveComponent.SetMaterial` _staticmesh 0 "/Game/Materials/MI_LaserAnimated_Red.MI_LaserAnimated_Red")
      (if (`self.IsDamageRadial`)
        (set `self.DamageType` "/Game/Blueprints/Weapons/DamageType_Explosion_RedTeam.DamageType_Explosion_RedTeam_C")
        (else
          (set `self.DamageType` "/Game/Blueprints/Weapons/Damage_RedTeam.Damage_RedTeam_C"))))
    (:`NewEnumerator1`
      (`PrimitiveComponent.SetMaterial` _staticmesh 0 "/Game/Materials/MI_LaserAnimated_Blue.MI_LaserAnimated_Blue")
      (if (`self.IsDamageRadial`)
        (set `self.DamageType` "/Game/Blueprints/Weapons/DamageType_Explosion_BlueTeam.DamageType_Explosion_BlueTeam_C")
        (else
          (set `self.DamageType` "/Game/Blueprints/Weapons/Damage_BlueTeam.Damage_BlueTeam_C"))))))