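; Test shield weapon that scales up a force field with pulsing audio while used and shrinks it on release, via multicast events.
; Heat timelines drive the material's Temperature, with overheat blocking activation until a penalty cooldown finishes; this graph never calls the heat events from firing.
; Construction sizes timelines from variables and applies team light color.
; Dropped shields self-destroy after a delay unless held; OnRep custom-color logic is disconnected.
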(event `self.ReceiveBeginPlay`
  ;[0.06432 1 0.1783] Begin Play
)

(event `StopNormalHeatTimeline`
  ;[1 1 1] Overheating
  (`TimelineComponent.SetNewTime` (`self.OverheatTimeline`) 0.0)
  (bind (_direction _temptime) (`Timeline|OverheatTimeline` :`NewTime` (+ (`self.CoolTime`) (`self.TimeTempPenaltyPerShot`)) :!via `Stop` :!label _label)
    (:`Update`
      (bind _output_get (set `self.CoolTime` _temptime))
      (`MaterialInstanceDynamic.SetScalarParameterValue` (`self.MaterialInstanceDynamic`) "Temperature" (`KismetMathLibrary.MapRangeClamped` _output_get 0.0 (`self.MaxPassiveCooldownTime`) 0.0 1.5)))
    (:`Finished`
      _))
  (if (`KismetMathLibrary.NearlyEqual_FloatFloat` _output_get (`self.MaxPassiveCooldownTime`) (`self.TimeTempPenaltyPerShot`))
    (`self.StopNormalHeatTimeline`)
    (set `self.IsOverheated` true)
    (bind (_direction_2 _cooldowntemp) (`Timeline|CooldownTimeline` :!via `ReverseFromEnd`)
      (:`Update`
        (`MaterialInstanceDynamic.SetScalarParameterValue` (`self.MaterialInstanceDynamic`) "Temperature" (`KismetMathLibrary.MapRangeClamped` _cooldowntemp 0.0 (`self.OverheatTimePenalty`) 0.0 1.5)))
      (:`Finished`
        (set `self.IsOverheated` false)
        (set `self.CoolTime` 0.0)))))

(event `CoolDown`
  ;[1 1 1] Overheating
  (goto _label :!via `Reverse`))

(event `AddHeat`
  ;[1 1 1] Overheating
  (goto _label :!via `SetNewTime`))

(event `StartFireWeapon_Multicast`
  ;[1 1 1] Fire Weapon
  (if (not (`self.IsOverheated`))
    (`AudioComponent.Play` (`self.AudioPulsate`) 0.0)
    (`AudioComponent.Play` (`self.AudioClick`) 0.0)
    (bind (_direction _animation) (`Timeline|Timeline_0` :!label _label_2)
      (:`Update`
        (`SceneComponent.SetRelativeScale3D` (`self.ForeField`) (`KismetMathLibrary.MakeVector` _animation _animation _animation))
        (`AudioComponent.SetVolumeMultiplier` (`self.AudioPulsate`) _animation)))))

(event `VRGripInterface.OnUsed`
  ;[1 1 1] Fire Weapon
  (`/Engine/EditorBlueprintResources/StandardMacros.IsValid` (`self.GetOwner`)
    (:`Is Valid`
      (`self.StartFireWeapon_Multicast`))
    (:`Is Not Valid`
      (`self.EndFireWeapon_Multicast`))))

(event `/Game/Blueprints/Grippable_Interaction.Use`)

(event `EndFireWeapon_Multicast`
  ;[1 1 1] Fire Weapon
  (`AudioComponent.Play` (`self.AudioClick`) 0.0)
  (`AudioComponent.Stop` (`self.AudioPulsate`))
  (goto _label_2 :!via `Reverse`))

(event `/Game/Blueprints/Grippable_Interaction.EndUse`)

(event `VRGripInterface.OnEndUsed`
  ;[1 1 1] Fire Weapon
  (`self.EndFireWeapon_Multicast`))

(event `/Game/Blueprints/Grippable_Interaction.Drop`
  ;[1 1 1] Fire Weapon
  (`KismetSystemLibrary.Delay` 10.0)
  (if (not (`self.IsHeld_0`))
    (`self.K2_DestroyActor`)))

(fn `OnRep_OwnersTeam`
  ;[1 1 1] Setup Custom Material Colors
  (bind _asvive_pawn_character (cast `/Game/VRExpansion/Vive/Vive_PawnCharacter` (`self.GetOwner`))))

(fn `UserConstructionScript`
  (bind _materialinstancedynamic (`self.MaterialInstanceDynamic`))
  (bind (_red _blue _friendly) (break `/Game/Blueprints/DATA/TeamColors` (`|Copy` (struct))))
  (bind _returnvalue (`KismetMaterialLibrary.CreateDynamicMaterialInstance` (`self.Material`)))
  (set `self.MaterialInstanceDynamic` _returnvalue)
  (`PrimitiveComponent.SetMaterial` (`self.StaticMeshComponent`) 0 (`self.MaterialInstanceDynamic`))
  (`TimelineComponent.SetTimelineLength` (`self.PostFireDelayTimeline`) (`self.PostFireDelay`))
  (`TimelineComponent.SetTimelineLength` (`self.OverheatTimeline`) (`self.MaxPassiveCooldownTime`))
  (`TimelineComponent.SetTimelineLength` (`self.CooldownTimeline`) (`self.OverheatTimePenalty`))
  (switch `/Game/Blueprints/DATA/Enum_Teams` (`self.OwnersTeam`)
    (:`NewEnumerator0`
      (`MaterialInstanceDynamic.SetVectorParameterValue` _materialinstancedynamic "LightColor" (`KismetMathLibrary.Conv_ColorToLinearColor` _red)))
    (:`NewEnumerator1`
      (`MaterialInstanceDynamic.SetVectorParameterValue` _materialinstancedynamic "LightColor" (`KismetMathLibrary.Conv_ColorToLinearColor` _blue)))
    (:`NewEnumerator2`
      (`MaterialInstanceDynamic.SetVectorParameterValue` _materialinstancedynamic "LightColor" (`KismetMathLibrary.Conv_ColorToLinearColor` _friendly)))))