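; Master VR helicopter vehicle with pilot, copilot and passenger seats, entered and exited via seat buttons with server-driven seating and navmesh-projected exits.
; A start button runs a timeline for rotors, sound and exhaust; hard impacts or rotor hits shut it down.
; On tick, grip levers drive chassis force and torque, with auto-hover and auto-leveling fallbacks, while a toggleable cable's end carries pickup actors.
; Tipped, empty helicopters destroy themselves after a delay.
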(event `Key|SpaceBar`
  (params (Key :type "Key Structure")))

(event `InputAxis|MoveForward`
  (params (AxisValue :type "Float (single-precision)"))
  ;[1 1 1] Non VR characters Control
  (if (and (not (`self.DriverIsInVR`)) (`self.IsLocallyControlled` (`self.LocalChar`)) (`KismetSystemLibrary.IsValid` (`.Character_2_802CB8CF418A6B0F37A1B09C520D5F08` (break `/Game/VRExpansion/Vive/Testing/Car/VehicleBP/Sedan/PassengerInfo` (`self.Driver`)))))
    _))

(event `InputAxis|MoveRight`
  (params (AxisValue :type "Float (single-precision)"))
  ;[1 1 1] Non VR characters Control
  (if (and (not (`self.DriverIsInVR`)) (`self.IsLocallyControlled` (`self.LocalChar`)) (`KismetSystemLibrary.IsValid` (`.Character_2_802CB8CF418A6B0F37A1B09C520D5F08` (break `/Game/VRExpansion/Vive/Testing/Car/VehicleBP/Sedan/PassengerInfo` (`self.Driver`)))))
    _))

(event `CharacterTakingControl`
  (params (Character :type "Character Object Reference") (IsTaking :type Boolean) (Attachment :type "SceneComponent Object Reference") (RelativeTransformToSeat :type "Transform Structure") (InitialCameraTransform :type "Transform Structure"))
  ;[1 1 1] Server sided setup of seating - also calls multicast to inform everyone that there is a new sitting client
  (`self.NotifyPlayerEnteredVehicle` Character IsTaking)
  (bind _asvrbase_character (cast `VRBaseCharacter` Character))
  (`VRBaseCharacter.Server_SetSeatedMode` _asvrbase_character Attachment IsTaking (`VRExpansionFunctionLibrary.Conv_TransformToTransformNetQuantize` RelativeTransformToSeat) (`VRExpansionFunctionLibrary.Conv_TransformToTransformNetQuantize` InitialCameraTransform) 40.0 20.0 true "C_MOVE_Walking")
  (if IsTaking
    (if (== Attachment (`self.PilotAttachment`))
      (bind _assteam_vr_player_controller (cast `/Game/VRExpansion/Vive/Steam_VR_Player_Controller` (`self.GetController` _asvrbase_character)))
      (set `self.DriverIsInVR` (`/Game/VRExpansion/Vive/Steam_VR_Player_Controller.HMDEnabled` _assteam_vr_player_controller)))))

(event `Key|MotionController_Left_Shoulder`
  (params (Key :type "Key Structure"))
  (bind _localchar (`self.LocalChar`))
  ;[1 1 1] Re-zero
  (:`Pressed`
    (`/Engine/EditorBlueprintResources/StandardMacros.IsValid` _localchar
      (:`Is Valid`
        (`VRBaseCharacter.Server_ReZeroSeating` :`self` _localchar)))))

(event `NotifyPlayerEnteredVehicle`
  (params (Character :type "Character Object Reference") (IsEntering :type Boolean))
  ;[1 1 1] Set up input binding - if only binding to driver we could run this owner only instead of multicast. But this car binds to everyones input
  (if (`self.IsLocallyControlled` Character)
    (bind _asvive_pawn_character (cast `/Game/VRExpansion/Vive/Vive_PawnCharacter` Character))
    (set `self.LocalChar` _asvive_pawn_character)
    (if IsEntering
      (bind _returnvalue (`self.GetController` _asvive_pawn_character))
      (`self.SetBindToInput` _returnvalue true)
      (add `VRBaseCharacter.OnSeatThreshholdChanged_Bind` _asvive_pawn_character (delegate `OnSeatedThresholdChanged`))
      (else
        (`self.SetBindToInput` _returnvalue)
        (remove `VRBaseCharacter.OnSeatThreshholdChanged_Bind` _asvive_pawn_character (delegate `OnSeatedThresholdChanged`))
        (if (`self.IsFadingCamera`) :!label _label
          (`PlayerCameraManager.StopCameraFade` (`GameplayStatics.GetPlayerCameraManager` 0))
          (set `self.IsFadingCamera` false))))))

(event `OnSeatedThresholdChanged`
  (params (bIsWithinThreshold :type Boolean) (ToThresholdScaler :type "Float (double-precision)"))
  ;[1 1 1] Optional camera darkening
  (if (`self.IsLocallyControlled`)
    (if bIsWithinThreshold
      (goto _label)
      (else
        (`PlayerCameraManager.SetManualCameraFade` :`self` (`GameplayStatics.GetPlayerCameraManager` 0) :`InFadeAmount` ToThresholdScaler)
        (set `self.IsFadingCamera` true)))))

(event `self.CableButton.OnButtonStateChanged`
  (params (ButtonState :type Boolean) (InteractingActor :type "Actor Object Reference") (InteractingComponent :type "PrimitiveComponent Object Reference"))
  (bind _cable (`self.Cable`))
  (bind _cablebutton (`self.CableButton`))
  (`SceneComponent.SetVisibility` _cable ButtonState false)
  (set `self.IsPickupCableActive` ButtonState)
  (if ButtonState
    (`PrimitiveComponent.SetMaterial` _cablebutton 0 "/Game/Materials/MasterMaterials/M_Button.M_Button")
    (`PrimitiveComponent.SetCollisionEnabled` _cable "QueryAndPhysics")
    (else
      (`PrimitiveComponent.SetMaterial` _cablebutton 0 "/Game/VRExpansion/Vive/Testing/Button/Button_Mat_Inst.Button_Mat_Inst")
      (`PrimitiveComponent.SetCollisionEnabled` _cable "NoCollision"))))

(event `self.ReceiveTick`
  (params (DeltaSeconds :type "Float (single-precision)"))
  ;[1 0.2083 0.2083] TICK 30hz Update Flight Controls
  (`|ExecutionSequence`
    (:`then_0`
      (if (`self.IsMotorReady`)
        (`self.UpdateGyroGuage`)
        (bind (_throttleposition _turnposition) (`self.GetThrottleTurnLever`))
        (bind (_forwardposition _sidewaysposition) (`self.GetLeanLever`))
        (`self.ApplySpecialEffects` _throttleposition)
        (`|ExecutionSequence`
          (:`then_0`
            (if (or (`VRLeverComponent.bIsHeld` (`self.ThrottleSteerLever`)) (not (== _throttleposition 0.0)))
              (`self.UpdateManualThrottleTurnControl` _throttleposition _turnposition)
              (else
                (`self.UpdateAutoHover`))))
          (:`then_1`
            (if (`VRLeverComponent.bIsHeld` (`self.LeanLever`))
              (`self.UpdateManualLeanControl` _forwardposition _sidewaysposition _turnposition)
              (else
                (`self.UpdateAutoLean` _turnposition))))
          (:`then_2`
            (if (`self.IsPickupCableActive`)
              (bind _hasgrabbedobject (`self.UpdatePickupBox`))
              (if _hasgrabbedobject
                (`/Engine/EditorBlueprintResources/StandardMacros.DoOnce` false :!label _label_2
                  (:`Completed`
                    (`PrimitiveComponent.SetMaterial` (`self.CableButton`) 0 "/Game/Materials/MasterMaterials/M_Master_SolidColor_Lit.M_Master_SolidColor_Lit")
                    (`GameplayStatics.PlaySoundAtLocation` "/Game/Audio/Wav/Blueprints_Scanner_Change05.Blueprints_Scanner_Change05" (`SceneComponent.K2_GetComponentLocation` (`self.Chassis`)) (struct) 1.0 1.0 0.0 null null null)))
                (else
                  (goto _label_2 :!via `Reset`))))))))
    (:`then_1`
      ;;[1 1 1] Remove Damaged Inactive
      (`KismetSystemLibrary.Delay` 5.0)
      (`/Engine/EditorBlueprintResources/StandardMacros.FlipFlop`
        (:`A`
          (if (< (.z (`SceneComponent.GetUpVector` (`self.Chassis`))) 0.5)
            (if (< (`self.PassengerCount`) 1)
              (`KismetSystemLibrary.Delay` 15.0)
              (if (< (`self.PassengerCount`) 1)
                (`self.K2_DestroyActor`)))))))))

(event `self.PilotExitButton.OnButtonStateChanged`
  (params (ButtonState :type Boolean) (InteractingActor :type "Actor Object Reference") (InteractingComponent :type "PrimitiveComponent Object Reference"))
  ;[0.4158 1 0.5126] Enter& Exit Triggers
  (`self.HandleExitButton` ButtonState (`self.PilotAttachment`) (`self.PilotExitLocation`) (`self.Driver`) (`self.PilotExitButton`)))

(event `self.CopilotExitButton.OnButtonStateChanged`
  (params (ButtonState :type Boolean) (InteractingActor :type "Actor Object Reference") (InteractingComponent :type "PrimitiveComponent Object Reference"))
  ;[0.4158 1 0.5126] Enter& Exit Triggers
  (`self.HandleExitButton` ButtonState (`self.CopilotAttachment`) (`self.CopilotExitLocation`) (`self.Copilot`) (`self.CopilotExitButton`)))

(event `self.TurretLever.OnWasUsed`
  ;[1 1 1] Turret
  (bind _isa (`/Engine/EditorBlueprintResources/StandardMacros.FlipFlop`)
    (:`A`
      _)
    (:`B`
      _))
  (`SceneComponent.SetVisibility` (`self.Lazer`) _isa false))

(event `self.PortsidePassengerExitButton.OnButtonStateChanged`
  (params (ButtonState :type Boolean) (InteractingActor :type "Actor Object Reference") (InteractingComponent :type "PrimitiveComponent Object Reference"))
  ;[0.4158 1 0.5126] Enter& Exit Triggers
  (`self.HandleExitButton` ButtonState (`self.PassengerPortside`) (`self.PassengarPortsideExitLocation`) (`self.PassengerLt`) (`self.PortsidePassengerExitButton`)))

(event `self.RotorGuide.OnComponentHit`
  (params (HitComponent :type "PrimitiveComponent Object Reference") (OtherActor :type "Actor Object Reference") (OtherComp :type "PrimitiveComponent Object Reference") (NormalImpulse :type "Vector Structure") (Hit :type "HitResult Structure (by ref)"))
  (bind _exhaustparticles (`self.ExhaustParticles`))
  (bind _motorsound (`self.MotorSound`))
  ;[1 1 1] Helicopter Disabled Chrashed
  (if (`self.IsMotorReady`)
    (`GameplayStatics.PlaySoundAtLocation` "/Game/Audio/Wav/SFX_Explosion1.SFX_Explosion1" (`SceneComponent.K2_GetComponentLocation` (`self.Chassis`)) (struct) 1.0 (`KismetMathLibrary.RandomFloatInRange` 0.85 1.2) 0.0 "/Game/Audio/SoundAttenuation_Normal.SoundAttenuation_Normal" "/Game/Audio/NormalSoundConcurrency.NormalSoundConcurrency" null :!label _label_3)
    ;[0.3575 1 0.7868] Start Stop the Engine
    (bind (_direction _motorstartup _soundoutput) (`Timeline|HelicopterStartSequence` :!via `Reverse` :!label _label_4)
      (:`Update`
        (`|ExecutionSequence`
          (:`then_0`
            (`/Engine/EditorBlueprintResources/StandardMacros.DoOnce` false :!label _label_5
              (:`Completed`
                (`AudioComponent.Play` _motorsound 0.0)
                (`AudioComponent.Play` (`self.RotorSound`) 0.0)
                (`ActorComponent.Activate` _exhaustparticles true)
                (`SceneComponent.SetVisibility` (`self.MainRotor`) true false)
                (`SceneComponent.SetVisibility` (`self.CockpitLight`) true false)
                (`SceneComponent.SetVisibility` (`self.RotorBlur`) false false)
                (set `self.HoverAltitude` 0.0))))
          (:`then_1`
            (`AudioComponent.SetPitchMultiplier` _motorsound _motorstartup)
            (`AudioComponent.SetPitchMultiplier` (`self.RotorSound`) _motorstartup)
            (`AudioComponent.SetVolumeMultiplier` _motorsound _soundoutput)
            (`AudioComponent.SetVolumeMultiplier` (`self.RotorSound`) _motorstartup)
            (bind _returnvalue (* _motorstartup (`self.RotorSpeedMultiplier`)))
            (`SceneComponent.K2_AddRelativeRotation` (`self.MainRotor`) (`KismetMathLibrary.MakeRotator` 0.0 0.0 _returnvalue) false false)
            (`SceneComponent.K2_AddRelativeRotation` (`self.RearRotor`) (`KismetMathLibrary.MakeRotator` _returnvalue) false false)
            (set `self.IsMotorReady` false))))
      (:`Finished`
        ;;[1 1 1] Completed or went back to the beginning
        (switch `ETimelineDirection` _direction
          (:`Forward`
            (set `self.IsMotorReady` true)
            (`SceneComponent.SetVisibility` (`self.MainRotor`) false false)
            (`SceneComponent.SetVisibility` (`self.RotorBlur`) true false)
            (set `self.CurrentRotorSpeed` 4.0)
            (goto _label_5 :!via `Reset`))
          (:`Backward`
            (`ActorComponent.Deactivate` _exhaustparticles)
            (`AudioComponent.Stop` (`self.RotorSound`))
            (`AudioComponent.Stop` (`self.MotorSound`))
            (`SceneComponent.SetVisibility` (`self.CockpitLight`) false false)
            (goto _label_5 :!via `Reset`)))))))

(event `self.Chassis.OnComponentHit`
  (params (HitComponent :type "PrimitiveComponent Object Reference") (OtherActor :type "Actor Object Reference") (OtherComp :type "PrimitiveComponent Object Reference") (NormalImpulse :type "Vector Structure") (Hit :type "HitResult Structure (by ref)"))
  ;[1 1 1] Helicopter Disabled Chrashed
  (if (> (`KismetMathLibrary.VSizeSquared` NormalImpulse) 729999998976.0)
    (goto _label_3)))

(event `self.StarboardPassengerExitButton.OnButtonStateChanged`
  (params (ButtonState :type Boolean) (InteractingActor :type "Actor Object Reference") (InteractingComponent :type "PrimitiveComponent Object Reference"))
  ;[0.4158 1 0.5126] Enter& Exit Triggers
  (`self.HandleExitButton` ButtonState (`self.PassengerStarboard`) (`self.PassengerStarboardExitLocation`) (`self.PassengerRt`) (`self.StarboardPassengerExitButton`)))

(event `self.StartButton.OnButtonStateChanged`
  (params (ButtonState :type Boolean) (InteractingActor :type "Actor Object Reference") (InteractingComponent :type "PrimitiveComponent Object Reference"))
  (bind _startbutton (`self.StartButton`))
  ;[0.3575 1 0.7868] Start Stop the Engine
  (if ButtonState
    (`PrimitiveComponent.SetMaterial` _startbutton 0 "/Game/Materials/MasterMaterials/M_Button.M_Button")
    (if (> (.z (`SceneComponent.GetUpVector` (`self.Chassis`))) 0.5)
      (goto _label_4)
      (else
        (`GameplayStatics.PlaySoundAtLocation` "/Game/Audio/Wav/S_LeverStop.S_LeverStop" (`SceneComponent.K2_GetComponentLocation` (`self.StartButton`)) (struct) 1.0 1.0 0.0 "/Game/Audio/CloseRangeSoundAttenuation.CloseRangeSoundAttenuation" "/Game/Audio/NormalSoundConcurrency.NormalSoundConcurrency" null)))
    (else
      (`PrimitiveComponent.SetMaterial` _startbutton 0 "/Game/VRExpansion/Vive/Testing/Button/Button_Mat_Inst.Button_Mat_Inst")
      (goto _label_4 :!via `Reverse`))))

(fn `AdvancedGripSettings`
  (returns (ReturnValue :type "BPAdvGripSettings Structure"))
  (return))

(fn `AllowsMultipleGrips`
  (returns (ReturnValue :type Boolean))
  (return false))

(fn `ApplySpecialEffects`
  (params (ThrottlePosition :type "Float (double-precision)"))
  ;[1 1 1] Effects
  (`AudioComponent.SetPitchMultiplier` (`self.MotorSound`) (+ (* ThrottlePosition -0.03) 1.0))
  (`AudioComponent.SetVolumeMultiplier` (`self.RotorSound`) (+ (* ThrottlePosition 0.5) 1.0))
  (`SceneComponent.K2_AddRelativeRotation` (`self.RotorBlur`) (`KismetMathLibrary.MakeRotator` 0.0 0.0 (`self.CurrentRotorSpeed`)) false false)
  (`SceneComponent.K2_AddRelativeRotation` (`self.RearRotor`) (`KismetMathLibrary.MakeRotator` 28.0) false false))

(fn `CheckSeatsForMissingButts`
  (returns (ButtIsMissing :type Boolean) (SeatNumber :type Integer))
  (for (_array_element _array_index) _
    (`/Engine/EditorBlueprintResources/StandardMacros.IsValid` null
      (:`Is Valid`
        (if (> (`KismetMathLibrary.VSize` (- (`self.K2_GetActorLocation` (break `/Game/VRExpansion/Vive/Testing/Car/VehicleBP/Sedan/PassengerInfo` _array_element)) (`SceneComponent.K2_GetComponentLocation` (`self.Chassis`)))) 500.0)
          (return true _array_index)))))
  (return false 0))

(fn `ClosestGripSlotInRange`
  (params (WorldLocation :type "Vector Structure") (bSecondarySlot :type Boolean) (CallingController :type "GripMotionControllerComponent Object Reference") (OverridePrefix :type Name))
  (returns (bHadSlotInRange :type Boolean) (SlotWorldTransform :type "Transform Structure"))
  (return false))

(fn `DenyGripping`
  (returns (ReturnValue :type Boolean))
  (return false))

(fn `GetExitTeleportLocation`
  (params (ExitMarker :type "SceneComponent Object Reference") (Character :type "VRBaseCharacter Object Reference"))
  (returns (LocationToTeleportTo :type "Vector Structure"))
  (bind _returnvalue (`SceneComponent.K2_GetComponentLocation` ExitMarker))
  (bind _projectedexitlocation (`self.ProjectedExitLocation`))
  (bind (_projectedlocation _returnvalue_2) (`NavigationSystemV1.K2_ProjectPointToNavigation` _returnvalue null null (400.0 400.0 200.0)))
  (bind _output_get (set `self.ProjectedExitLocation` _projectedlocation))
  (if (not (and (!= _returnvalue _output_get) _returnvalue_2 (!= _projectedlocation (0.0 0.0 0.0) :`ErrorTolerance` 0.001)))
    (set `self.ProjectedExitLocation` (`VRBaseCharacter.GetVRLocation` Character)))
  (bind _outhit (`KismetSystemLibrary.LineTraceSingleForObjects` _projectedexitlocation (+ _projectedexitlocation (0.0 0.0 -200.0)) (`|MakeArray` "ObjectTypeQuery1" :!type "EObjectTypeQuery Enum") false (`|MakeArray` (`self.Pilot`) :!type "Actor Object Reference"))) ; Trace down to find a valid location for player to stand at (original NavMesh location is offset upwards, so we must find the actual floor)
  (bind (_bblockinghit _binitialoverlap _time _distance _location _impactpoint) (`GameplayStatics.BreakHitResult` _outhit))
  (return (`KismetMathLibrary.SelectVector` _impactpoint _returnvalue _bblockinghit)))

(fn `GetGripScripts`
  (returns (ArrayReference :type "Array of VRGripScriptBase Object Reference") (ReturnValue :type Boolean))
  (return _ false))

(fn `GetGripStiffnessAndDamping`
  (returns (GripStiffnessOut :type "Float (double-precision)") (GripDampingOut :type "Float (double-precision)"))
  (return 0.0 0.0))

(fn `GetLeanLever`
  (returns (ForwardPosition :type "Float (double-precision)") (SidewaysPosition :type "Float (double-precision)"))
  (bind _leanlever (`self.LeanLever`))
  (bind _leverlimitpositive (`VRLeverComponent.LeverLimitPositive` _leanlever))
  (bind (_relativerotation_roll _relativerotation_pitch) (`KismetMathLibrary.BreakRotator` (`SceneComponent.RelativeRotation` _leanlever)))
  (return (/ _relativerotation_roll _leverlimitpositive) (/ _relativerotation_pitch _leverlimitpositive)))

(fn `GetPrimaryGripType`
  (params (bIsSlot :type Boolean))
  (returns (ReturnValue :type "EGripCollisionType Enum"))
  (return "InteractiveCollisionWithPhysics"))

(fn `GetThrottleTurnLever`
  (returns (ThrottlePosition :type "Float (double-precision)") (TurnPosition :type "Float (double-precision)"))
  (bind _throttlesteerlever (`self.ThrottleSteerLever`))
  (bind _leverlimitpositive (`VRLeverComponent.LeverLimitPositive` _throttlesteerlever))
  (return (/ (.roll (`SceneComponent.RelativeRotation` _throttlesteerlever)) _leverlimitpositive) (/ (.pitch (`SceneComponent.RelativeRotation` _throttlesteerlever)) _leverlimitpositive)))

(fn `GripBreakDistance`
  (returns (ReturnValue :type "Float (double-precision)"))
  (return 0.0))

(fn `GripLateUpdateSetting`
  (returns (ReturnValue :type "EGripLateUpdateSettings Enum"))
  (return "LateUpdatesAlwaysOn"))

(fn `GripMovementReplicationType`
  (returns (ReturnValue :type "EGripMovementReplicationSettings Enum"))
  (return "KeepOriginalMovement"))

(fn `HandleExitButton`
  (params (ButtonState :type Boolean) (Attachment :type "SceneComponent Object Reference") (ExitLocation :type "SceneComponent Object Reference") (PassengerInfo :type "/Game/VRExpansion/Vive/Testing/Car/VehicleBP/Sedan/PassengerInfo Structure") (Button :type "VRButtonComponent Object Reference"))
  (returns (Success :type Boolean))
  (bind _locallastinteractingcomponent (`VRButtonComponent.LocalLastInteractingComponent` Button))
  (`/Engine/EditorBlueprintResources/ActorMacros.Switch Has Authority`
    (:`Authority`
      (if ButtonState
        (`/Engine/EditorBlueprintResources/StandardMacros.IsValid` (`.Character_2_802CB8CF418A6B0F37A1B09C520D5F08` (break `/Game/VRExpansion/Vive/Testing/Car/VehicleBP/Sedan/PassengerInfo` PassengerInfo))
          (:`Is Not Valid`
            (`/Engine/EditorBlueprintResources/StandardMacros.IsValid` _locallastinteractingcomponent
              (:`Is Valid`
                (bind _asvrbase_character (cast `VRBaseCharacter` (`ActorComponent.GetOwner` _locallastinteractingcomponent)))
                (`self.SitPlayerDown` Attachment _asvrbase_character PassengerInfo)))))
        (else
          (`self.StandPlayerUp` Attachment ExitLocation PassengerInfo)))
      (return true))))

(fn `IsHeld`
  (returns (HoldingControllers :type "Array of BPGripPair Structure") (bIsHeld :type Boolean))
  (return _ false))

(fn `RequestsSocketing`
  (returns (ParentToSocketTo :type "SceneComponent Object Reference") (OptionalSocketName :type Name) (RelativeTransform :type "Transform_NetQuantize Structure") (ReturnValue :type Boolean))
  (return null "None" (struct) false))

(fn `SecondaryGripType`
  (returns (ReturnValue :type "ESecondaryGripType Enum"))
  (return "SG_None"))

(fn `SimulateOnDrop`
  (returns (ReturnValue :type Boolean))
  (return false))

(fn `SitPlayerDown`
  (params (Attachment :type "SceneComponent Object Reference") (Pilot :type "VRBaseCharacter Object Reference") (SeatNumber :type "/Game/VRExpansion/Vive/Testing/Car/VehicleBP/Sedan/PassengerInfo Structure"))
  (bind _vrreplicatedcamera (`VRBaseCharacter.VRReplicatedCamera` Pilot))
  (`/Engine/EditorBlueprintResources/StandardMacros.IsValid` Pilot
    (:`Is Valid`
      (setmembers `/Game/VRExpansion/Vive/Testing/Car/VehicleBP/Sedan/PassengerInfo` :`StructRef` SeatNumber :`Character` Pilot :`InitialRelativeLocation` (`SceneComponent.RelativeLocation` _vrreplicatedcamera))
      (`self.CharacterTakingControl` Pilot true Attachment (`SceneComponent.GetRelativeTransform` _vrreplicatedcamera) (`KismetMathLibrary.MakeTransform` (0.0 0.0 0.0)))
      (`self.SetActorTickEnabled` true)
      (`/Engine/EditorBlueprintResources/StandardMacros.IncrementInt` (`self.PassengerCount`)
        (:`  `
          (if (== Attachment (`self.PilotAttachment`))
            (`self.SetOwner` Pilot)
            (set `self.LocalChar` Pilot)))))))

(fn `StandPlayerUp`
  (params (Attachment :type "SceneComponent Object Reference") (ExitLocation :type "SceneComponent Object Reference") (PassengerInfo :type "/Game/VRExpansion/Vive/Testing/Car/VehicleBP/Sedan/PassengerInfo Structure"))
  (bind ((`Character_2_802CB8CF418A6B0F37A1B09C520D5F08` _character)) (break `/Game/VRExpansion/Vive/Testing/Car/VehicleBP/Sedan/PassengerInfo` PassengerInfo))
  (`/Engine/EditorBlueprintResources/StandardMacros.IsValid` _character
    (:`Is Valid`
      (`self.GetExitTeleportLocation` ExitLocation _character)
      (`self.CharacterTakingControl` _character false Attachment)
      (`/Engine/EditorBlueprintResources/StandardMacros.DecrementInt` (`self.PassengerCount`)
        (:`  `
          (setmembers `/Game/VRExpansion/Vive/Testing/Car/VehicleBP/Sedan/PassengerInfo` :`StructRef` PassengerInfo :`Character` _character))))
    (:`Is Not Valid`
      _))
  (if (== Attachment (`self.PilotAttachment`))
    (`self.SetOwner` null)
    (set `self.LocalChar` _character)))

(fn `TeleportBehavior`
  (returns (ReturnValue :type "EGripInterfaceTeleportBehavior Enum"))
  (return "TeleportAllComponents"))

(fn `UpdateAutoHover`
  (bind _chassis (`self.Chassis`))
  (bind _z (.z (`SceneComponent.K2_GetComponentLocation` _chassis)))
  ;[1 1 1] Auto Hover
  (`PrimitiveComponent.AddForce` _chassis (* (`SceneComponent.GetUpVector` _chassis) (+ (`self.BaseHoverForce`) (* (- (`self.HoverAltitude`) _z) 900.0))) "None" false)
  (if (> (`KismetMathLibrary.Abs` (- (`self.HoverAltitude`) _z)) (`self.AutoHoverAltitudeSwitchTolerance`))
    (set `self.HoverAltitude` _z)))

(fn `UpdateAutoLean`
  (params (TurnPosition :type "Float (double-precision)"))
  (bind _chassis (`self.Chassis`))
  (bind _autoleancorrectionforce (`self.AutoLeanCorrectionForce`))
  (bind (_relativerotation_roll _relativerotation_pitch) (`KismetMathLibrary.BreakRotator` (`SceneComponent.RelativeRotation` _chassis)))
  (`PrimitiveComponent.AddTorqueInDegrees` _chassis (`KismetMathLibrary.GreaterGreater_VectorRotator` (`KismetMathLibrary.MakeVector` (* _relativerotation_roll _autoleancorrectionforce) (* _relativerotation_pitch _autoleancorrectionforce) (* TurnPosition (`self.TurnForce`))) (`SceneComponent.K2_GetComponentRotation` _chassis)) "None" true))

(fn `UpdateGyroGuage`
  (bind (_relativerotation_roll _relativerotation_pitch _relativerotation_yaw) (`KismetMathLibrary.BreakRotator` (`SceneComponent.RelativeRotation` (`self.Chassis`))))
  (`SceneComponent.K2_SetWorldRotation` (`self.LevelGuage`) (`KismetMathLibrary.MakeRotator` 0.0 0.0 _relativerotation_yaw) false false))

(fn `UpdateManualLeanControl`
  (params (ForwardAmount :type "Float (double-precision)") (SidewaysAmount :type "Float (double-precision)") (TurnPosition :type "Float (double-precision)"))
  (bind _leanforce (`self.LeanForce`))
  (bind _chassis (`self.Chassis`))
  ;[1 1 1] Tilt and Auto level
  (`PrimitiveComponent.AddTorqueInDegrees` _chassis (`KismetMathLibrary.GreaterGreater_VectorRotator` (`KismetMathLibrary.MakeVector` (* ForwardAmount _leanforce) (* SidewaysAmount _leanforce) (* TurnPosition (`self.TurnForce`))) (`SceneComponent.RelativeRotation` _chassis)) "None" true))

(fn `UpdateManualThrottleTurnControl`
  (params (ThrottlePosition :type "Float (double-precision)") (TurnPosition :type "Float (double-precision)"))
  (bind _chassis (`self.Chassis`))
  (bind _z (.z (`SceneComponent.K2_GetComponentLocation` _chassis)))
  ;[1 1 1] Lift
  (`PrimitiveComponent.AddForce` _chassis (* (`SceneComponent.GetUpVector` _chassis) (- (+ (* ThrottlePosition (`self.MotorForceMultiplier`)) (`self.BaseHoverForce`)) (* _z 20.0))) "None" false)
  (set `self.HoverAltitude` _z))

(fn `UpdatePickupBox`
  (returns (HasGrabbedObject :type Boolean))
  (bind _pickupbox (`self.PickupBox`))
  (bind _locations (`CableComponent.GetCableParticleLocations` (`self.Cable`)))
  (bind _output (`|GetArrayItem` _locations (- (`KismetArrayLibrary.Array_Length` _locations) 1)))
  (`SceneComponent.K2_SetWorldLocation` _pickupbox _output false false)
  (bind _asbp_helicopter_pickup_master (cast `/Game/Blueprints/Targets/BP_HelicopterPickupMaster` (`|GetArrayItem` (`PrimitiveComponent.GetOverlappingActors` _pickupbox "/Game/Blueprints/Targets/BP_HelicopterPickupMaster.BP_HelicopterPickupMaster_C")))
    (:`then`
      (`SceneComponent.K2_SetWorldLocation` (`Actor.RootComponent` _asbp_helicopter_pickup_master) _output false false)
      (return true))
    (:`CastFailed`
      (return false))))

(fn `UserConstructionScript`
  (bind (_returnvalue_x _returnvalue_y _returnvalue_z) (`KismetMathLibrary.BreakVector` (`SceneComponent.K2_GetComponentLocation` (`self.Chassis`))))
  (set `self.HoverAltitude` _returnvalue_z))