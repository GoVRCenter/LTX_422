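; Master door Blueprint that opens for overlapping pawns, optionally restricted to player and bot characters on its team, with team-colored material.
; Authority-side sensor overlaps trigger opening or a denial sound, while a timeline slides the door vertically with audio.
; Once open, it powers linked electrical targets.
; Auto-return logic is disconnected, CheckForPawns closes only without loitering pawns, and Server_CloseDoor calls OpenDoor rather than CloseDoor.
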(event `CheckForPawns`
  ;[1 1 1] Check for loiterers before closing
  (if (`self.IsOpen`)
    (if (`KismetArrayLibrary.Array_IsValidIndex` (`PrimitiveComponent.GetOverlappingActors` (`self.DoorSensor`) "/Script/Engine.Pawn"))
      (`KismetSystemLibrary.PrintString` "Grr")
      (else
        (`self.Server_CloseDoor`)
        (`KismetSystemLibrary.PrintString` "CLOSE!")))))

(event `self.DoorSensor.OnComponentBeginOverlap`
  (params (OverlappedComponent :type "PrimitiveComponent Object Reference") (OtherActor :type "Actor Object Reference") (OtherComp :type "PrimitiveComponent Object Reference") (OtherBodyIndex :type Integer) (bFromSweep :type Boolean) (SweepResult :type "HitResult Structure (by ref)"))
  ;[1 1 1] Door Functionality and Replication
  (`/Engine/EditorBlueprintResources/ActorMacros.Switch Has Authority`
    (:`Authority`
      (`KismetSystemLibrary.PrintString` "ENTER" true true (struct :`G` 0.66 :`B` 1.0 :`A` 1.0) 22.0)
      (if (or (`self.IsOpen`) (`self.IsLocked`))
        _
        (elif (`self.AllowTeamOnly`)
          (bind _asvive_pawn_character (cast `/Game/VRExpansion/Vive/Vive_PawnCharacter` OtherActor)
            (:`then`
              (if (`|EnumEquality` (`/Game/VRExpansion/Vive/Vive_PawnCharacter.Team` _asvive_pawn_character) (`self.Team`))
                (`self.Server_OpenDoor` :!label _label)
                (else
                  (`self.DenyDoor` :!label _label_2))))
            (:`CastFailed`
              (bind _asai_master_bot (cast `/Game/Blueprints/AI/AI_Master_Bot` OtherActor))
              (if (`|EnumEquality` (`/Game/Blueprints/AI/AI_Master_Bot.Team` _asai_master_bot) (`self.Team`))
                (goto _label)
                (else
                  (goto _label_2)))))
          (else
            (cast `Pawn` OtherActor)
            (goto _label)))))))

(event `OpenDoor`
  ;[1 1 1] Door Functionality and Replication
  (if (not (`self.IsOpen`))
    (set `self.IsMoving` true)
    (`AudioComponent.Play` (`self.Audio`) 0.0)
    (bind (_direction _movement) (`Timeline|Timeline_Animation` :!label _label_3)
      (:`Update`
        (`SceneComponent.K2_SetRelativeLocation` (`self.Door`) (`KismetMathLibrary.MakeVector` 0.0 0.0 _movement) false false))
      (:`Finished`
        (set `self.IsMoving` false)
        (bind _output_get (set `self.IsOpen` (`|EnumEquality` _direction "Forward")))
        (if _output_get
          (for _array_element (`self.ElectricalTargets`)
            (bind _aselectrical_object (cast `/Game/VRExpansion/Vive/Testing/Button/ElectricalObject` _array_element))
            (`/Game/Blueprints/Spawners/BP_AI_Spawner.CurrentStateChange` _aselectrical_object self true 0.0)))))))

(event `CloseDoor`
  ;[1 1 1] Door Functionality and Replication
  (if (`self.IsOpen`)
    (set `self.IsMoving` true)
    (`AudioComponent.Play` (`self.Audio`) 0.0)
    (goto _label_3 :!via `Reverse`)))

(event `Server_OpenDoor`
  ;[1 1 1] Door Functionality and Replication
  (if (`self.IsLocked`)
    (`self.DenyDoor`)
    (else
      (`self.OpenDoor`))))

(event `DenyDoor`
  ;[1 1 1] Door Functionality and Replication
  (`GameplayStatics.PlaySoundAtLocation` "/Game/Audio/Wav/S_LeverStop.S_LeverStop" (`self.K2_GetActorLocation`) (struct) 1.0 1.0 0.0 "/Game/Audio/SoundAttenuation_Normal.SoundAttenuation_Normal" null null))

(event `Server_CloseDoor`
  ;[1 1 1] Door Functionality and Replication
  (if (`self.IsLocked`)
    (`self.DenyDoor`)
    (else
      (`self.OpenDoor`))))

(event `self.DoorSensor.OnComponentEndOverlap`
  (params (OverlappedComponent :type "PrimitiveComponent Object Reference") (OtherActor :type "Actor Object Reference") (OtherComp :type "PrimitiveComponent Object Reference") (OtherBodyIndex :type Integer))
  ;[1 1 1] Door Functionality and Replication
  (`/Engine/EditorBlueprintResources/ActorMacros.Switch Has Authority`))

(fn `OnRep_IsOpen`
  (if (`self.IsOpen`)
    (`self.Server_CloseDoor`)
    (else
      (`self.Server_OpenDoor`))))

(fn `UserConstructionScript`
  (bind _door (`self.Door`))
  (switch `/Game/Blueprints/DATA/Enum_Teams` (`self.Team`)
    (:`NewEnumerator0`
      (`PrimitiveComponent.SetMaterial` _door 0 "/Game/Materials/MI_Concrete_Light_Tiles_Red.MI_Concrete_Light_Tiles_Red"))
    (:`NewEnumerator1`
      (`PrimitiveComponent.SetMaterial` _door 0 "/Game/Materials/MI_Concrete_Light_Tiles_Blue.MI_Concrete_Light_Tiles_Blue"))))