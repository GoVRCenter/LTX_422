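; VR game instance that manages multiplayer sessions and holds lobby settings and red/blue team scores.
; Hosting destroys the old session, creates one with LAN forced on, and opens the selected map as a listen server; joining also clears the old session first.
; AddToScore and OnRep handlers push scores to GameMode_Gameplay.
; A save-slot check only sets a flag, and network/travel error handlers print strings from stubs that return empty text.
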(event `SaveGameCheck`
  ;[1 1 1] Check for a save Game Slot Name
  (bind _returnvalue (`GameplayStatics.DoesSaveGameExist` (`self.Save_PlayerSettings`)))
  (bind _output_get (set `self.HasSaveGame` _returnvalue))
  (if _output_get
    _))

(event `SaveLobbySettings`
  (params (NumberOfPlayers :type Integer) (IsLAN :type Boolean) (ServerName :type Text) (SelectedMap :type Name) (PlayToScore :type Integer))
  (bind _returnvalue (`GameplayStatics.GetPlayerController` 0))
  ;[1 1 1] Launch Lobby
  (set `self.MaxNumOfPlayers` NumberOfPlayers)
  (set `self.SelectedMap` SelectedMap)
  (set `self.PlayToScore` PlayToScore)
  (set `self.ServerName` ServerName)
  (`DestroySessionCallbackProxy.DestroySession` _returnvalue
    (:`OnSuccess`
      _)
    (:`OnFailure`
      _))
  (`CreateSessionCallbackProxy.CreateSession` _returnvalue (`self.MaxNumOfPlayers`) true
    (:`OnSuccess`
      (`GameplayStatics.OpenLevel` (`self.SelectedMap`) true "listen"))))

(event `JoinServer`
  (params (SessionToJoin :type "BlueprintSessionResult Structure"))
  (bind _returnvalue (`GameplayStatics.GetPlayerController` 0))
  ;[1 1 1] Join Server
  (`self.DestroySessionCaller` _returnvalue)
  (`JoinSessionCallbackProxy.JoinSession` _returnvalue SessionToJoin
    (:`OnFailure`
      (`KismetSystemLibrary.PrintString` "Failed to join session"))))

(event `self.HandleNetworkError`
  (params (FailureType :type "ENetworkFailure Enum" :default "NetDriverAlreadyExists") (bIsServer :type Boolean))
  ;[1 1 1] Network Errors
  (if bIsServer
    _
    (else
      _))
  (`KismetSystemLibrary.PrintString` (`self.NetworkErrorToString` FailureType)))

(event `self.HandleTravelError`
  (params (FailureType :type "ETravelFailure Enum" :default "NoLevel"))
  ;[1 1 1] Network Errors
  (`KismetSystemLibrary.PrintString` (`self.TravelErrorToString` FailureType)))

(event `DestroySessionCaller`
  (params (PlayerController :type "PlayerController Object Reference"))
  ;[1 1 1] End Old Session
  (`DestroySessionCallbackProxy.DestroySession` PlayerController))

(event `AddToScore`
  (params (ScoringTeam :type "/Game/Blueprints/DATA/Enum_Teams Enum" :default "NewEnumerator0") (AmountScored :type Integer))
  ;[1 1 1] Score
  (switch `/Game/Blueprints/DATA/Enum_Teams` ScoringTeam
    (:`NewEnumerator0`
      (set `self.RedTeamScore` (+ (`self.RedTeamScore`) AmountScored)))
    (:`NewEnumerator1`
      (set `self.BlueTeamScore` (+ (`self.BlueTeamScore`) AmountScored))))
  (bind _asgame_mode_gameplay (cast `/Game/Blueprints/Gameplay/GameMode_Gameplay` (`GameplayStatics.GetGameMode`)))
  (`/Game/Blueprints/Gameplay/GameMode_Gameplay.UpdateScore` _asgame_mode_gameplay (`self.RedTeamScore`) (`self.BlueTeamScore`)))

(fn `NetworkErrorToString`
  (params (FailureType :type "ENetworkFailure Enum" :default "NetDriverAlreadyExists"))
  (returns (OutSTring :type String))
  (return ""))

(fn `OnRep_BlueTeamScore`
  (bind _asgame_mode_gameplay (cast `/Game/Blueprints/Gameplay/GameMode_Gameplay` (`GameplayStatics.GetGameMode`)))
  (set `/Game/Blueprints/Gameplay/GameMode_Gameplay.BlueTeamScore` (`self.BlueTeamScore`) _asgame_mode_gameplay))

(fn `OnRep_RedTeamScore`
  (bind _asgame_mode_gameplay (cast `/Game/Blueprints/Gameplay/GameMode_Gameplay` (`GameplayStatics.GetGameMode`)))
  (set `/Game/Blueprints/Gameplay/GameMode_Gameplay.RedTeamScore` (`self.RedTeamScore`) _asgame_mode_gameplay))

(fn `TravelErrorToString`
  (params (FailureType :type "ETravelFailure Enum" :default "NoLevel"))
  (returns (OutString :type String))
  (return ""))