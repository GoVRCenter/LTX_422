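; Gameplay player controller for a team game that supports both VR and desktop FPS players.
; BeginPlay and Respawn detect the HMD and request spawning from GameMode_Gameplay; Die credits the opposing team and respawns after a delay.
; SpawnCharacter possesses a Vive or FPS pawn at a random team-tagged start, compensating for HMD yaw and position, then applies display console commands.
; Helper functions load and save player info, including team, through a save slot.
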(event `InitHMD`
  (params (bHasHMD :type Boolean))
  ;[1 1 1] Set up Console Commands
  (if bHasHMD
    ;;[1 1 1] Vr Console Commands
    (`KismetSystemLibrary.ExecuteConsoleCommand` "vr.bEnableStereo true" self) ; Oculus Only
    (`KismetSystemLibrary.ExecuteConsoleCommand` "sg.ResolutionQuality 100" self)
    (`KismetSystemLibrary.ExecuteConsoleCommand` "r.screenpercentage 100" null)
    (`KismetSystemLibrary.ExecuteConsoleCommand` "vr.PixelDensity 1" null)
    (else
      ;;[1 1 1] Non VR Console Commands
      (`KismetSystemLibrary.ExecuteConsoleCommand` "vr.bEnableStereo false" self) ; Oculus Only
      (`KismetSystemLibrary.ExecuteConsoleCommand` "r.setres 1024x768w" null))))

(event `SetTeam`
  (params (Team :type "/Game/Blueprints/DATA/Enum_Teams Enum" :default "NewEnumerator0"))
  ;[1 1 1] Set Team
  (set `self.Team` Team))

(event `Die`
  (params (Team :type "/Game/Blueprints/DATA/Enum_Teams Enum" :default "NewEnumerator0"))
  (bind _returnvalue (`self.K2_GetPawn`))
  (bind _returnvalue_2 (`GameplayStatics.GetGameMode`))
  ;[1 1 1] Client Death, Score, and Respawn
  (switch `/Game/Blueprints/DATA/Enum_Teams` Team
    (:`NewEnumerator0`
      (bind _asgame_mode_gameplay (cast `/Game/Blueprints/Gameplay/GameMode_Gameplay` _returnvalue_2))
      (`/Game/Blueprints/Gameplay/GameMode_Gameplay.UpdateScore` _asgame_mode_gameplay 0 1))
    (:`NewEnumerator1`
      (bind _asgame_mode_gameplay_2 (cast `/Game/Blueprints/Gameplay/GameMode_Gameplay` _returnvalue_2))
      (`/Game/Blueprints/Gameplay/GameMode_Gameplay.UpdateScore` _asgame_mode_gameplay_2 1 0))
    (:`NewEnumerator2`
      _))
  (`KismetSystemLibrary.Delay` 5.0)
  (`/Engine/EditorBlueprintResources/StandardMacros.IsValid` _returnvalue
    (:`Is Valid`
      (`self.UnPossess`)
      (`self.K2_DestroyActor` _returnvalue))
    (:`Is Not Valid`
      _))
  (`self.Respawn`))

(event `SpawnCharacter`
  (bind (_devicerotation _deviceposition) (`HeadMountedDisplayFunctionLibrary.GetOrientationAndPosition`))
  (bind _spawnpoints (`self.SpawnPoints`))
  (bind _spawnpoint (`self.SpawnPoint`))
  (bind _spawnpoints_2 (`self.SpawnPoints`))
  (bind _returnvalue (`KismetArrayLibrary.Array_Length` _spawnpoints_2))
  (bind _returnvalue_2 (`KismetArrayLibrary.Array_Length` _spawnpoints))
  ;[1 1 1] Spawn and possess a VR or FPS pawn
  (`KismetArrayLibrary.Array_Clear` (`self.SpawnPoints`))
  (if (`self.IsInVR`)
    (bind _outactors (`GameplayStatics.GetAllActorsOfClass` "/Script/Engine.PlayerStart"))
    (for _array_element _outactors
      (if (== (`PlayerStart.PlayerStartTag` _array_element) (`KismetStringLibrary.Conv_StringToName` (`|GetEnumeratorNameAsString` (`self.Team`))))
        (`KismetArrayLibrary.Array_Add` (`self.SpawnPoints`) _array_element)))
    (if (> _returnvalue_2 0)
      (set `self.SpawnPoint` (`|GetArrayItem` _spawnpoints (`KismetMathLibrary.RandomIntegerInRange` 0 (- _returnvalue_2 1))))
      (else
        (set `self.SpawnPoint` (`|GetArrayItem` _outactors (`KismetMathLibrary.RandomIntegerInRange` 0 (- (`KismetArrayLibrary.Array_Length` _outactors) 1))))))
    (bind _returnvalue_3 (`|SpawnActorFromClass` "/Game/VRExpansion/Vive/Vive_PawnCharacter.Vive_PawnCharacter_C" (`KismetMathLibrary.ComposeTransforms` (`KismetMathLibrary.InvertTransform` (`KismetMathLibrary.MakeTransform` (`self.OffsetSpawnByCapsuleHalfHeight` _spawnpoint (`KismetMathLibrary.MakeVector` (.x _deviceposition) (.y _deviceposition))) (`VRExpansionFunctionLibrary.GetHMDPureYaw` _devicerotation))) (`self.GetTransform` _spawnpoint)) "AdjustIfPossibleButAlwaysSpawn" "OverrideRootScale" self (`self.Team`) true null))
    (`self.Possess` _returnvalue_3)
    (`self.InitHMD` true)
    (else
      (bind _outactors_2 (`GameplayStatics.GetAllActorsOfClass` "/Script/Engine.PlayerStart"))
      (for _array_element_2 _outactors_2
        (if (== (`PlayerStart.PlayerStartTag` _array_element_2) (`KismetStringLibrary.Conv_StringToName` (`|GetEnumeratorNameAsString` (`self.Team`))))
          (`KismetArrayLibrary.Array_Add` (`self.SpawnPoints`) _array_element_2)))
      (if (> _returnvalue 0)
        (set `self.SpawnPoint` (`|GetArrayItem` _spawnpoints_2 (`KismetMathLibrary.RandomIntegerInRange` 0 (- _returnvalue 1))))
        (else
          (set `self.SpawnPoint` (`|GetArrayItem` _outactors_2 (`KismetMathLibrary.RandomIntegerInRange` 0 (- (`KismetArrayLibrary.Array_Length` _outactors_2) 1))))))
      (bind _returnvalue_4 (`|SpawnActorFromClass` "/Game/VRExpansion/Vive/FPS_VivePawnCharacter.FPS_VivePawnCharacter_C" (`self.GetTransform` (`self.SpawnPoint`)) "AlwaysSpawn" "OverrideRootScale" self (`self.Team`) false null))
      (`self.Possess` _returnvalue_4)
      (`self.InitHMD` false))))

(event `Respawn`
  (bind (_devicerotation _deviceposition) (`HeadMountedDisplayFunctionLibrary.GetOrientationAndPosition`))
  (bind _returnvalue (`self.K2_GetPawn`))
  ;[1 1 1] Respawn
  (`/Engine/EditorBlueprintResources/StandardMacros.IsValid` _returnvalue
    (:`Is Valid`
      (`self.UnPossess`)
      (`self.K2_DestroyActor` _returnvalue))
    (:`Is Not Valid`
      _))
  ;[0.1574 1 0] Begin Play
  (set `self.IsInVR` (and (`VRExpansionFunctionLibrary.GetIsHMDConnected`) (`VRExpansionFunctionLibrary.IsInVREditorPreviewOrGame`)) :!label _label)
  (if (`self.IsInVR`)
    (set `self.IsInVR` true)
    (`/Engine/EditorBlueprintResources/ActorMacros.Switch Has Authority`
      (:`Authority`
        (`KismetSystemLibrary.ExecuteConsoleCommand` "vr.bEnableStereo true" self) ; Forces stereo here as it hasn't been done yet for server
        (if (`HeadMountedDisplayFunctionLibrary.HasValidTrackingPosition`)
          _
          (else
            _)))
      (:`Remote`
        _))
    (`PlayerCameraManager.StartCameraFade` :`self` (`GameplayStatics.GetPlayerCameraManager` 0) :`FromAlpha` 1.0 :`Duration` 3.0) ; Remove fade now
    (else
      (`PlayerCameraManager.StartCameraFade` :`self` (`GameplayStatics.GetPlayerCameraManager` 0) :`FromAlpha` 1.0 :`Duration` 3.0) ; Remove fade now
    ))
  (bind _asgame_mode_gameplay (cast `/Game/Blueprints/Gameplay/GameMode_Gameplay` (`GameplayStatics.GetGameMode`)))
  (`/Game/Blueprints/Gameplay/GameMode_Gameplay.SpawnPlayerController` _asgame_mode_gameplay self _devicerotation (`KismetMathLibrary.MakeVector` (.x _deviceposition) (.y _deviceposition)) (`self.Team`) (`self.IsInVR`)))

(event `self.ReceiveBeginPlay`
  ;[0.1574 1 0] Begin Play
  (goto _label))

(fn `CheckLoadGame`
  (returns (CreatedSaveGame :type Boolean) (LoadedTeam :type "/Game/Blueprints/DATA/Enum_Teams Enum"))
  (bind _save_playersettings (`self.Save_PlayerSettings`))
  (bind _playerinfo (`self.PlayerInfo`))
  (bind _returnvalue (`GameplayStatics.DoesSaveGameExist` _save_playersettings))
  (if _returnvalue
    (bind _returnvalue_2 (`GameplayStatics.LoadGameFromSlot` _save_playersettings))
    (bind _asplayer_save_game (cast `/Game/Blueprints/Gameplay/PlayerSaveGame` _returnvalue_2)
      (:`then`
        (bind _output_get (set `self.PlayerSaveGame_Ref` _asplayer_save_game))
        (bind (_s_playerinfo_name _s_playerinfo_thumbnail _s_playerinfo_class _s_playerinfo_status _s_playerinfo_colors _s_playerinfo_team _s_playerinfo_ping) (break `/Game/Blueprints/DATA/PlayerInfo` (`/Game/Blueprints/Gameplay/PlayerSaveGame.S_PlayerInfo` _output_get)))
        (setmembers `/Game/Blueprints/DATA/PlayerInfo` :`StructRef` (`self.PlayerInfo`) :`Name` _s_playerinfo_name :`thumbnail` _s_playerinfo_thumbnail :`Class` _s_playerinfo_class :`Status` _s_playerinfo_status :`Colors` _s_playerinfo_colors :`Team` _s_playerinfo_team :`Ping` _s_playerinfo_ping)
        (bind _output_get_2 (set `self.Team` _s_playerinfo_team))
        (`KismetSystemLibrary.PrintString` (`KismetStringLibrary.Concat_StrStr` "Loaded game and spawning player from: " (`|GetEnumeratorNameAsString` _output_get_2) " Team"))
        (return false _output_get_2))
      (:`CastFailed`
        _)))
  (`/Engine/EditorBlueprintResources/StandardMacros.IsValid` (`self.PlayerSaveGame_Ref`)
    (:`Is Valid`
      (`KismetSystemLibrary.PrintString` "Updated From Save Game")
      (bind _output_get_3 (set `/Game/Blueprints/Gameplay/PlayerSaveGame.S_PlayerInfo` _playerinfo (`self.PlayerSaveGame_Ref`)))
      (bind _output_get_4 (set `self.Team` (`.Team_23_10D5D6CC48F70BACBB94FE9806A5D8E4` (break `/Game/Blueprints/DATA/PlayerInfo` _output_get_3))))
      (return true _output_get_4))
    (:`Is Not Valid`
      (bind _returnvalue_3 (`GameplayStatics.CreateSaveGameObject` "/Game/Blueprints/Gameplay/PlayerSaveGame.PlayerSaveGame_C"))
      (bind _output_get_5 (set `self.PlayerSaveGame_Ref` _returnvalue_3))
      (set `/Game/Blueprints/Gameplay/PlayerSaveGame.S_PlayerInfo` _playerinfo _output_get_5)
      (`GameplayStatics.SaveGameToSlot` _output_get_5 _save_playersettings)
      (`KismetSystemLibrary.PrintString` "Created New Save Game Slot and Saved Game")
      (set `self.Team` "NewEnumerator2")
      (return true "NewEnumerator0"))))

(fn `OffsetSpawnByCapsuleHalfHeight`
  (params (PlayerStart :type "PlayerStart Object Reference") (HMDOffset :type "Vector Structure"))
  (returns (OffsetVectorFinal :type "Vector Structure"))
  (bind _ascapsule_collision (cast `CapsuleComponent` (`Actor.RootComponent` PlayerStart)))
  (return (`KismetMathLibrary.MakeVector` (.x HMDOffset) (.y HMDOffset) (`CapsuleComponent.CapsuleHalfHeight` _ascapsule_collision))))

(fn `OnRep_Team`)

(fn `SaveGame`
  (returns (WasSuccessful :type Boolean))
  (bind _playersavegame_ref (`self.PlayerSaveGame_Ref`))
  (bind _save_playersettings (`self.Save_PlayerSettings`))
  (bind (_playerinfo_name _playerinfo_thumbnail _playerinfo_class _playerinfo_status _playerinfo_colors _playerinfo_team _playerinfo_ping) (break `/Game/Blueprints/DATA/PlayerInfo` (`self.PlayerInfo`)))
  (set `self.PlayerInfo` (make `/Game/Blueprints/DATA/PlayerInfo` _playerinfo_name _playerinfo_thumbnail _playerinfo_class _playerinfo_status _playerinfo_colors (`self.Team`) _playerinfo_ping))
  (`/Engine/EditorBlueprintResources/StandardMacros.IsValid` _playersavegame_ref
    (:`Is Valid`
      (set `/Game/Blueprints/Gameplay/PlayerSaveGame.S_PlayerInfo` (`self.PlayerInfo`) _playersavegame_ref)
      (bind _returnvalue (`GameplayStatics.SaveGameToSlot` _playersavegame_ref _save_playersettings))
      (return _returnvalue))
    (:`Is Not Valid`
      (bind _returnvalue_2 (`GameplayStatics.DoesSaveGameExist` _save_playersettings))
      (if _returnvalue_2
        (bind _returnvalue_3 (`GameplayStatics.LoadGameFromSlot` _save_playersettings))
        (bind _asplayer_save_game (cast `/Game/Blueprints/Gameplay/PlayerSaveGame` _returnvalue_3))
        (bind _output_get (set `self.PlayerSaveGame_Ref` _asplayer_save_game))
        (set `/Game/Blueprints/Gameplay/PlayerSaveGame.S_PlayerInfo` (`self.PlayerInfo`) _output_get)
        (bind _returnvalue_4 (`GameplayStatics.SaveGameToSlot` _output_get _save_playersettings))
        (return _returnvalue_4)
        (else
          (bind _returnvalue_5 (`GameplayStatics.CreateSaveGameObject` "/Game/Blueprints/Gameplay/PlayerSaveGame.PlayerSaveGame_C"))
          (set `self.PlayerSaveGame_Ref` _returnvalue_5))))))

(fn `UserConstructionScript`)