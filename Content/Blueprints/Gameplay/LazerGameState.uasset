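; Game state for a two-team match that keeps the Red and Blue team scores with RepNotify.
; AddToScore adds points to the scoring team, then passes both totals to GameMode_Gameplay through UpdateScore.
; Each OnRep function also copies its score into GameMode_Gameplay, doing nothing where that game mode cast fails, as on clients.
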(event `AddToScore`
  (params (ScoringTeam :type "/Game/Blueprints/DATA/Enum_Teams Enum" :default "NewEnumerator0") (AmountScored :type Integer))
  ;[1 1 1] Score
  (switch `/Game/Blueprints/DATA/Enum_Teams` ScoringTeam
    (:`NewEnumerator0`
      (set `self.RedTeamScore` (+ (`self.RedTeamScore`) AmountScored)))
    (:`NewEnumerator1`
      (set `self.BlueTeamScore` (+ (`self.BlueTeamScore`) AmountScored))))
  (bind _asgame_mode_gameplay (cast `/Game/Blueprints/Gameplay/GameMode_Gameplay` (`GameplayStatics.GetGameMode`)))
  (`/Game/Blueprints/Gameplay/GameMode_Gameplay.UpdateScore` _asgame_mode_gameplay (`self.RedTeamScore`) (`self.BlueTeamScore`)))

(fn `OnRep_BlueTeamScore`
  (bind _asgame_mode_gameplay (cast `/Game/Blueprints/Gameplay/GameMode_Gameplay` (`GameplayStatics.GetGameMode`)))
  (set `/Game/Blueprints/Gameplay/GameMode_Gameplay.BlueTeamScore` (`self.BlueTeamScore`) _asgame_mode_gameplay))

(fn `OnRep_RedTeamScore`
  (bind _asgame_mode_gameplay (cast `/Game/Blueprints/Gameplay/GameMode_Gameplay` (`GameplayStatics.GetGameMode`)))
  (set `/Game/Blueprints/Gameplay/GameMode_Gameplay.RedTeamScore` (`self.RedTeamScore`) _asgame_mode_gameplay))

(fn `UserConstructionScript`)