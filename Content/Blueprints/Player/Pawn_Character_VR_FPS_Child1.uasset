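; Child of the VR FPS player character that adds flat-screen look controls for when the player is not in VR.
; LookRight feeds controller yaw, while LookUp accumulates an inverted, scaled and clamped pitch value that rotates the VROrigin component directly instead of using controller pitch.
; BeginPlay and the construction script only call the parent.
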(event `self.ReceiveBeginPlay`
  (`parent.ReceiveBeginPlay`))

(event `InputAxis|LookRight`
  (params (AxisValue :type "Float (single-precision)"))
  ;[1 1 1] FPS Turning AIming control
  (if (not (`self.IsInVR`))
    (`self.AddControllerYawInput` AxisValue)))

(event `InputAxis|LookUp`
  (params (AxisValue :type "Float (single-precision)"))
  ;[1 1 1] FPS Turning AIming control
  (if (not (`self.IsInVR`))
    (bind _output_get (set `self.PointerAimingFPS` (`KismetMathLibrary.FClamp` (+ (* AxisValue -2.0) (`self.PointerAimingFPS`)) -90.0 90.0)))
    (`SceneComponent.K2_SetRelativeRotation` (`self.VROrigin`) (`KismetMathLibrary.MakeRotator` 0.0 _output_get) false false)))

(fn `UserConstructionScript`
  (`parent.UserConstructionScript`))