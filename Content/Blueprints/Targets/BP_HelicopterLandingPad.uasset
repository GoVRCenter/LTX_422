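; BP_HelicopterLandingPad is a landing pad target that uses a spotlight to signal when a VRVehiclePawn arrives slowly enough.
; On overlap begin it checks the pawn's speed once and turns the SpotLight green if it is below a fixed threshold.
; When the pawn leaves, a delay runs before the light is set to red, with no check for re-entry in the meantime.
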(event `self.ReceiveActorBeginOverlap`
  (params (OtherActor :type "Actor Object Reference"))
  (bind _asvrvehicle_pawn (cast `VRVehiclePawn` OtherActor))
  (if (< (`KismetMathLibrary.VSize` (`self.GetVelocity` _asvrvehicle_pawn)) 450.0)
    (`LightComponent.SetLightColor` (`self.SpotLight`) (struct :`R` 0.1875 :`G` 1.0 :`B` 0.252029 :`A` 1.0) true)))

(event `self.ReceiveActorEndOverlap`
  (params (OtherActor :type "Actor Object Reference"))
  (cast `VRVehiclePawn` OtherActor)
  (`KismetSystemLibrary.Delay` 15.0)
  (`LightComponent.SetLightColor` (`self.SpotLight`) (struct :`R` 1.0 :`G` 0.2 :`B` 0.2 :`A` 1.0) true))

(fn `UserConstructionScript`)