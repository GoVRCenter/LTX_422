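; Team capture zone that Red and Blue players and bots contest to earn score for their side.
; A server timer counts overlapping characters into a signed, replicated TeamDominance, displayed as text.
; Dominance drives a color timeline into a material parameter collection, reversing to neutralize, and completing a capture spawns a coin with effects.
; A second timer periodically awards the owning team points in LazerGameState, scaled by dominance.
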(event `/Game/VRExpansion/Vive/Testing/Button/ElectricalObject.CurrentStateChange`
  (params (CurrentProvider :type "Object Object Reference") (ElectricalState :type Boolean) (CurrentFlow :type "Float (single-precision)"))
  (`/Engine/EditorBlueprintResources/StandardMacros.DoOnce` false
    (:`Completed`
      (`KismetSystemLibrary.Delay` 30.0))))

(event `self.ReceiveBeginPlay`
  ;[0 1 0.1211] Begin Play
  (if (`KismetSystemLibrary.IsServer`)
    (`KismetSystemLibrary.K2_SetTimerDelegate` (delegate `UpdateCaptureStatus`) 1.0 true)
    (`KismetSystemLibrary.K2_SetTimerDelegate` (delegate `UpdateScore`) 5.0 true)))

(event `UpdateScore`
  (bind _returnvalue (`GameplayStatics.GetGameState`))
  ;[1 1 1] Check Scoring
  (if (`self.RedCaptured`)
    (bind _aslazer_game_state (cast `/Game/Blueprints/Gameplay/LazerGameState` _returnvalue))
    (`/Game/Blueprints/Gameplay/LazerGameState.AddToScore` _aslazer_game_state "NewEnumerator0" (+ (`KismetMathLibrary.Abs_Int` (`self.TeamDominance`)) 1))
    (elif (`self.BlueCaptured`)
      (bind _aslazer_game_state_2 (cast `/Game/Blueprints/Gameplay/LazerGameState` _returnvalue))
      (`/Game/Blueprints/Gameplay/LazerGameState.AddToScore` _aslazer_game_state_2 "NewEnumerator1" (+ (`self.TeamDominance`) 1)))))

(event `UpdateCaptureStatus`
  (bind _teamdominance (`self.TeamDominance`))
  (bind _teamdominance_2 (`self.TeamDominance`))
  (bind _teamdominance_3 (`self.TeamDominance`))
  (bind (_red _blue _friendly) (break `/Game/Blueprints/DATA/TeamColors` (`|Copy` (struct))))
  ;[1 1 1] Determine Team dominance
  (set `self.IsPlayerDetected` false)
  (set `self.TeamDominance` 0)
  (for _array_element (`PrimitiveComponent.GetOverlappingActors` (`self.Box`) "/Script/Engine.Character")
    (bind _asvive_pawn_character (cast `/Game/VRExpansion/Vive/Vive_PawnCharacter` _array_element)
      (:`then`
        (set `self.IsPlayerDetected` true)
        (switch `/Game/Blueprints/DATA/Enum_Teams` (`/Game/VRExpansion/Vive/Vive_PawnCharacter.Team` _asvive_pawn_character) ; Red team is negative numbers, blue is positive
          (:`NewEnumerator0`
            (set `self.TeamDominance` (- _teamdominance 1)))
          (:`NewEnumerator1`
            (set `self.TeamDominance` (+ _teamdominance 1)))))
      (:`CastFailed`
        (bind _asai_master_bot (cast `/Game/Blueprints/AI/AI_Master_Bot` _array_element))
        (set `self.IsPlayerDetected` true)
        (switch `/Game/Blueprints/DATA/Enum_Teams` (`/Game/Blueprints/AI/AI_Master_Bot.Team` _asai_master_bot) ; Red team is negative numbers, blue is positive
          (:`NewEnumerator0`
            (set `self.TeamDominance` (- _teamdominance_2 1)))
          (:`NewEnumerator1`
            (set `self.TeamDominance` (+ _teamdominance_2 1)))))))
  ;[1 1 1] Fade Color depending on Team dominance
  (if (`self.IsPlayerDetected`)
    (if (> _teamdominance_3 0)
      (set `self.BlueDominant` true)
      (set `self.RedDominant` false)
      (if (`self.BlueCaptured`)
        _
        (elif (`self.RedCaptured`)
          (bind (_direction _timer) (`Timeline|ColorMixTimeline` :`NewTime` 8.0 :!via `Reverse` :!label _label)
            (:`Update`
              (`self.UpdateDominance` _timer))
            (:`Finished`
              (if (`|EnumEquality` _direction "Forward")
                (if (`self.BlueDominant`)
                  (set `self.BlueCaptured` true)
                  (set `self.RedCaptured` false)
                  (else
                    (set `self.RedCaptured` true)
                    (set `self.BlueCaptured` false)))
                (`|SpawnActorFromClass` "/Game/Blueprints/PowerUps/BP_Pickup_Coin.BP_Pickup_Coin_C" (`KismetMathLibrary.MakeTransform` (+ (0.0 0.0 400.0) (`self.K2_GetActorLocation`))) "Undefined" "OverrideRootScale" null true null)
                (`self.PlayEffects`)
                (else
                  (set `self.RedCaptured` false)
                  (set `self.BlueCaptured` false)
                  (set `self.BlueDominant` false)
                  (set `self.RedDominant` false)))))
          (else
            (set `self.TargetColor` (`KismetMathLibrary.Conv_ColorToLinearColor` _blue))
            (goto _label))))
      (elif (< _teamdominance_3 0)
        (set `self.BlueDominant` false)
        (set `self.RedDominant` true)
        (if (`self.RedCaptured`)
          _
          (elif (`self.BlueCaptured`)
            (goto _label :!via `Reverse`)
            (else
              (set `self.TargetColor` (`KismetMathLibrary.Conv_ColorToLinearColor` _red))
              (goto _label))))
        (else
          (set `self.BlueDominant` false)
          (set `self.RedDominant` false)
          (if (not (or (`self.RedCaptured`) (`self.BlueCaptured`))) :!label _label_2
            (goto _label :!via `Reverse`)))))
    (else
      (goto _label_2))))

(event `UpdateDominance`
  (params (Dominance :type "Float (double-precision)"))
  ;[1 1 1] UpdateClients
  (`KismetMaterialLibrary.SetVectorParameterValue` "/Game/Materials/ParameterCollections/MCP_WinningTeamColor.MCP_WinningTeamColor" "WinningTeam" (`KismetMathLibrary.LinearColorLerp` (`self.DefaultColor`) (`self.TargetColor`) Dominance)))

(event `PlayEffects`
  (bind _returnvalue (`SceneComponent.K2_GetComponentLocation` (`self.Box`)))
  ;[1 1 1] UpdateClients
  (`GameplayStatics.PlaySoundAtLocation` "/Game/Audio/Wav/SFX_Success_1.SFX_Success_1" _returnvalue (struct) 1.0 1.0 0.0 "/Game/Audio/SoundAttenuation_Normal.SoundAttenuation_Normal" "/Game/Audio/NormalSoundConcurrency.NormalSoundConcurrency" null)
  (`GameplayStatics.SpawnEmitterAtLocation` "/Game/Particles/P_Treasure_Burst.P_Treasure_Burst" _returnvalue))

(fn `OnRep_TeamDominance`
  (`TextRenderComponent.K2_SetText` (`self.TextRender`) (`KismetTextLibrary.Conv_IntToText` (`self.TeamDominance`))))

(fn `UserConstructionScript`
  (set `self.DefaultColor` (`KismetMathLibrary.Conv_ColorToLinearColor` (`.Friendly_11_5F4186CA4D24271DBBC0F98C6D326B7C` (break `/Game/Blueprints/DATA/TeamColors` (`|Copy` (struct)))))))