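; AI spawner that pads a team with bots to make up for missing players, running only on the server.
; On a state change, a looping timer with a randomized interval counts same-team Vive pawns against the team size.
; An empty or invalid slot within that shortfall in the bot array triggers a spawn at a random nearby point, passing team and patrol path to the new bot.
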(event `/Game/VRExpansion/Vive/Testing/Button/ElectricalObject.CurrentStateChange`
  (params (CurrentProvider :type "Object Object Reference") (ElectricalState :type Boolean) (CurrentFlow :type "Float (single-precision)"))
  ;[1 1 1] Begin Play
  (if (`KismetSystemLibrary.IsServer`)
    (if (> (`self.TeamSize`) 0)
      (`KismetSystemLibrary.K2_SetTimerDelegate` (delegate `SpawnNewAI`) (`KismetMathLibrary.RandomFloatInRange` 2.5 3.0) true))))

(event `SpawnNewAI`
  ;[1 1 1] Should we spawn another bot to pad the team?
  (`self.CheckLiveBots`)
  (if (`self.SpawnAnotherBot`)
    (bind _returnvalue (`|SpawnActorFromClass` "/Game/Blueprints/AI/AI_Master_Bot.AI_Master_Bot_C" (`KismetMathLibrary.MakeTransform` (`KismetMathLibrary.RandomPointInBoundingBox` (`self.K2_GetActorLocation`) (400.0 400.0 0.0))) "Undefined" "OverrideRootScale" null (`self.TeamToSpawn`) (`self.PatrolPath`) null))
    (`KismetArrayLibrary.Array_Add` (`self.AIBots`) _returnvalue)
    (set `self.SpawnAnotherBot` false)))

(event `CheckLiveBots`
  (bind _aibots (`self.AIBots`))
  (bind _teamsize (`self.TeamSize`))
  (bind _returnvalue (`KismetMathLibrary.Clamp` (- _teamsize (`self.TeamTotal`)) 0 (- _teamsize 1)))
  ;[1 1 1] Check alive bots and accomidate for number of players on the same team.
  (bind _outactors (`GameplayStatics.GetAllActorsOfClass` "/Game/VRExpansion/Vive/Vive_PawnCharacter.Vive_PawnCharacter_C"))
  (set `self.TeamTotal` 0)
  (for _array_element _outactors
    (if (`|EnumEquality` (`/Game/VRExpansion/Vive/Vive_PawnCharacter.Team` _array_element) (`self.TeamToSpawn`))
      (set `self.TeamTotal` (+ (`self.TeamTotal`) 1))))
  (if (> _returnvalue 0)
    (for _index (range (+ _returnvalue 1))
      (`/Engine/EditorBlueprintResources/StandardMacros.IsValid` (`|GetArrayItem` _aibots _index)
        (:`Is Not Valid`
          (`KismetArrayLibrary.Array_Remove` _aibots _index)
          (set `self.SpawnAnotherBot` true))))))

(fn `UserConstructionScript`)